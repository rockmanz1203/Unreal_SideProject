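; GameManager is a level setup actor that spawns the game's enemy, UI manager and blocks when play begins.
; On BeginPlay it spawns a scaled-up BP_Muffin, passes it as Enemy to a newly spawned BP_UIManager, and stores that manager.
; It then spawns five Block actors at hardcoded locations and injects the stored UI manager into each through SetUIManager.
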(event EventBeginPlay
  (bind _returnvalue (Game|SpawnActorfromClass "/Game/MuffinWar/Characters/Muffin/Blueprints/BP_Muffin.BP_Muffin_C" (Math|Transform|MakeTransform "209.000000,920.000000,210.000000" "0, 0, 0" "2.000000,2.000000,2.000000") "Undefined" 0 0))
  (bind _returnvalue_2 (Game|SpawnActorfromClass "/Game/UI/BP_UIManager.BP_UIManager_C" (Math|Transform|MakeTransform "0, 0, 0" "0, 0, 0" "1,1,1") "Undefined" 0 _returnvalue 0))
  (bind _output_get (Variables|Default|SetBP_UIManager _returnvalue_2)) ; 產生完自己也存一份起來，\n看看之後能不能配給動態產生的box
  (Utilities|FlowControl|Sequence
    (:then_0
      (bind _returnvalue_3 (Game|SpawnActorfromClass "/Game/Blueprints/Block.Block_C" (Math|Transform|MakeTransform "-300.000000,-300.000000,300.000000" "0, 0, 0" "1,1,1") "Undefined" 0 0))
      (Default|SetUIManager _returnvalue_3 _output_get))
    (:then_1
      (bind _returnvalue_4 (Game|SpawnActorfromClass "/Game/Blueprints/Block.Block_C" (Math|Transform|MakeTransform "-970.000000,-300.000000,300.000000" "0, 0, 0" "1,1,1") "Undefined" 0 0))
      (Default|SetUIManager _returnvalue_4 _output_get))
    (:then_2
      (bind _returnvalue_5 (Game|SpawnActorfromClass "/Game/Blueprints/Block.Block_C" (Math|Transform|MakeTransform "-720.000000,-120.000000,340.000000" "0, 0, 0" "1,1,1") "Undefined" 0 0))
      (Default|SetUIManager _returnvalue_5 _output_get))
    (:then_3
      (bind _returnvalue_6 (Game|SpawnActorfromClass "/Game/Blueprints/Block.Block_C" (Math|Transform|MakeTransform "-720.000000,-300.000000,300.000000" "0, 0, 0" "1,1,1") "Undefined" 0 0))
      (Default|SetUIManager _returnvalue_6 _output_get))
    (:then_4
      (bind _returnvalue_7 (Game|SpawnActorfromClass "/Game/Blueprints/Block.Block_C" (Math|Transform|MakeTransform "-720.000000,170.000000,280.000000" "0, 0, 0" "1,1,1") "Undefined" 0 0))
      (Default|SetUIManager _returnvalue_7 _output_get))))

(event Collision|EventActorBeginOverlap
  (params (OtherActor :type Actor%20Object%20Reference)))

(event EventTick
  (params (DeltaSeconds :type Float%20%28single-precision%29)))

(fn ConstructionScript)