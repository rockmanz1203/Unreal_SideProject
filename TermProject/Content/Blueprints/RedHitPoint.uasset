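; RedHitPoint is an aim-point marker actor that shows where the player's gun is pointing.
; Every Tick, UpdateAimPoint runs a Visibility line trace 5000 units forward from the player's GunLoaction component.
; It moves its root to the hit location without checking whether the trace hit anything.
; A debug print and a look-at-player rotation are present but never run.
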(event EventBeginPlay)

(event Collision|EventActorBeginOverlap
  (params (OtherActor :type Actor%20Object%20Reference)))

(event EventTick
  (params (DeltaSeconds :type Float%20%28single-precision%29))
  (CallFunction|UpdateAimPoint))

(fn ConstructionScript)

(fn UpdateAimPoint
  (bind _player (Variables|Default|GetPlayer))
  (bind _gunloaction (Variables|/Game/ThirdPersonBP/Blueprints/ThirdPersonCharacter.ThirdPersonCharacter_C|GetGunLoaction _player))
  (bind _returnvalue (Transformation|GetWorldLocation _gunloaction))
  (bind (_outhit _returnvalue_2) (Collision|LineTraceByChannel _returnvalue (+ _returnvalue (* (Math|Vector|RotateVector (Math|Vector|GetForwardVector _gunloaction) "0.000000,0.000000, 0") 5e+03)) "TraceTypeQuery1" false 0 "None"))
  (Transformation|SetWorldLocation (Variables|Default|GetDefaultSceneRoot) (.Location (Collision|BreakHitResult _outhit)) false false))